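; Player controller for human players that puts the Stats widget on screen and registers pawn ownership.
; BeginPlay branches on authority: the authority side creates the widget only if a controlled pawn is valid, while remote clients create it unconditionally.
; Remote clients also call a server event that sets the controller as owner of its controlled pawn.
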(event `self.ReceiveBeginPlay`
  (`/Engine/EditorBlueprintResources/ActorMacros.Switch Has Authority`
    (:`Authority`
      (`/Engine/EditorBlueprintResources/StandardMacros.IsValid` (`self.K2_GetPawn`)
        (:`Is Valid`
          (bind _returnvalue (`|CreateWidget` "/Game/Player/UI/Stats.Stats_C" self))
          (`UserWidget.AddToViewport` _returnvalue 0))))
    (:`Remote`
      (`self.Server_AddOwner`)
      (bind _returnvalue_2 (`|CreateWidget` "/Game/Player/UI/Stats.Stats_C" self))
      (`UserWidget.AddToViewport` _returnvalue_2 0))))

(event `Server_AddOwner`
  (`self.SetOwner` (`self.K2_GetPawn`) self))

(fn `UserConstructionScript`)